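; BP_Player is the player Blueprint that hooks grab input up to its Grabber.
; On BeginPlay it casts its controller to PlayerController and adds the IMC_InputMapping Enhanced Input context to the local player subsystem.
; The IA_Grab action calls Grab on the Grabber when it starts and Release when it completes, giving hold-to-grab control.
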(event Input|EnhancedActionEvents|EnhancedInputActionIA_Grab
  (params (ActionValue :type Boolean) (ElapsedSeconds :type Float%20%28double-precision%29) (TriggeredSeconds :type Float%20%28double-precision%29) (InputAction :type Input%20Action%20Object%20Reference :default "/Game/Input/IA_Grab.IA_Grab"))
  (bind _grabber (Variables|Default|GetGrabber))
  (:Started
    (Class|Grabber|Grab _grabber))
  (:Completed
    (Class|Grabber|Release _grabber)))

(event EventBeginPlay
  ;[1 1 1] Setup Input Mapping Context
  (bind _asplayer_controller (Utilities|Casting|CastToPlayerController (Pawn|GetController)))
  (Utilities|IsValid (PlayerController|LocalPlayerSubsystems|GetEnhancedInputLocalPlayerSubsystem _asplayer_controller)
    (:Is%20Valid
      (Input|AddMappingContext (PlayerController|LocalPlayerSubsystems|GetEnhancedInputLocalPlayerSubsystem _asplayer_controller) "/Game/Input/IMC_InputMapping.IMC_InputMapping" 0 "(bIgnoreAllPressedKeysUntilRelease=True,bForceImmediately=False,bNotifyUserSettings=False)"))))

(fn ConstructionScript
  (|CallParentFunction))